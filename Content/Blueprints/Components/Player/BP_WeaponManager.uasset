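; Player weapon manager component that spawns, stores and switches the character's weapons by slot.
; CreateWeapon attaches each spawn to the character and files it as main, secondary, melee, special or grenade.
; Client-named events drive selection and scrolling, which cycles only main, secondary and melee, to set CurrentWeapon.
; On non-server machines, CurrentWeapon's RepNotify returns the previous weapon to the character and attaches the new one to the visible mesh's weapon socket.
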(event `self.ReceiveBeginPlay`
  (bind _asbp_player_character (cast `/Game/Blueprints/Player/BP_PlayerCharacter` (`self.GetOwner`)))
  (set `self.Character` _asbp_player_character))

(event `SelectWeaponFromClient`
  (params (Type :type "/Game/Data/Enums/E_WeaponType Enum"))
  ;[1 1 1] Switch weapons
  (`self.SelectWeapon` Type))

(event `ScrollWeaponFromClient`
  (params (Next :type Boolean))
  ;[1 1 1] Switch weapons
  (`self.ScrollWeapon` Next))

(fn `CreateWeapon`
  (params (Class :type "/Game/Blueprints/Weapons/BP_WEapon Class Reference"))
  (returns (Weapon :type "/Game/Blueprints/Weapons/BP_WEapon Object Reference"))
  (locals (L_Weapon :type "/Game/Blueprints/Weapons/BP_WEapon Object Reference"))
  (bind _l_weapon (`local.L_Weapon`))
  (bind _character (`self.Character`))
  (bind _returnvalue (`|SpawnActorFromClass` Class (`KismetMathLibrary.MakeTransform` (0.0 0.0 0.0)) "AlwaysSpawn" "OverrideRootScale" (`Pawn.GetController` _character) _character))
  (bind _output_get (set `local.L_Weapon` _returnvalue))
  (switch `/Game/Data/Enums/E_WeaponType` (`/Game/Blueprints/Weapons/BP_WEapon.WeaponType` _output_get)
    (:`NewEnumerator0`
      (set `self.MainWeapon` _l_weapon))
    (:`NewEnumerator1`
      (set `self.SecondWeapon` _l_weapon))
    (:`NewEnumerator2`
      (`KismetArrayLibrary.Array_Add` (`self.Specials`) _l_weapon))
    (:`NewEnumerator3`
      (`KismetArrayLibrary.Array_Add` (`self.Grenades`) _l_weapon))
    (:`NewEnumerator4`
      (set `self.MeleeWeapon` (cast `/Game/Blueprints/Weapons/BP_MeleeWeapon` _l_weapon :!pure true))))
  (`Actor.K2_AttachToActor` (`local.L_Weapon`) (`self.Character`) "None" "SnapToTarget" "SnapToTarget" "KeepRelative" true)
  (return (`local.L_Weapon`)))

(fn `OnRep_CurrentWeapon`
  (if (not (`KismetSystemLibrary.IsServer`))
    (bind _clientweaponattached (`self.ClientWeaponAttached`)
      (:`then`
        (`Actor.K2_AttachToActor` _clientweaponattached (`self.Character`) "None" "SnapToTarget" "SnapToTarget" "KeepRelative" true))
      (:`else`
        _))
    (`Actor.K2_AttachToComponent` (`self.CurrentWeapon`) (`/Game/Blueprints/Player/BP_PlayerCharacter.GetVisibleMesh` (`self.Character`)) "Skt_Weapon" "KeepRelative" "KeepRelative" "KeepRelative" true)
    (set `self.ClientWeaponAttached` (`self.CurrentWeapon`))
    (`/Game/Blueprints/Libs/BP_Functions_Debug.PrintMessage` "Weapon attached" (struct :`G` 1.0 :`B` 0.577141 :`A` 1.0) 3.0)))

(fn `ScrollWeapon`
  (params (Next :type Boolean))
  (bind _weapontype (`/Game/Blueprints/Weapons/BP_WEapon.WeaponType` (`self.CurrentWeapon`)))
  (if Next
    (switch `/Game/Data/Enums/E_WeaponType` _weapontype
      (:`NewEnumerator0`
        (`self.SelectWeapon` "NewEnumerator1"))
      (:`NewEnumerator1`
        (`self.SelectWeapon` "NewEnumerator4"))
      (:`NewEnumerator4`
        (`self.SelectWeapon` "NewEnumerator0")))
    (else
      (switch `/Game/Data/Enums/E_WeaponType` _weapontype
        (:`NewEnumerator0`
          (`self.SelectWeapon` "NewEnumerator4"))
        (:`NewEnumerator1`
          (`self.SelectWeapon` "NewEnumerator0"))
        (:`NewEnumerator4`
          (`self.SelectWeapon` "NewEnumerator1"))))))

(fn `SelectWeapon`
  (params (Type :type "/Game/Data/Enums/E_WeaponType Enum") (Index :type Integer))
  (returns (Weapon :type "/Game/Blueprints/Weapons/BP_WEapon Object Reference"))
  (bind _returnvalue (select `/Game/Data/Enums/E_WeaponType` Type :`NewEnumerator0` (`self.MainWeapon`) :`NewEnumerator1` (`self.SecondWeapon`) :`NewEnumerator2` (`KismetArrayLibrary.Array_Get` (`self.Specials`) Index) :`NewEnumerator3` (`KismetArrayLibrary.Array_Get` (`self.Grenades`) Index) :`NewEnumerator4` (`self.MeleeWeapon`) :!type "/Game/Blueprints/Weapons/BP_WEapon Object Reference"))
  (`/Engine/EditorBlueprintResources/StandardMacros.IsValid` _returnvalue
    (:`Is Valid`
      (bind _output_get (set `self.CurrentWeapon` _returnvalue))
      (return _output_get))
    (:`Is Not Valid`
      (return (`self.CurrentWeapon`)))))