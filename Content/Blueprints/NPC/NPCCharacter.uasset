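; NPC character Blueprint that raises an alarm when it is damaged by the player.
; AnyDamage calls the parent handler, then calls Alarm if InstigatedBy, normally a Controller, equals the player character at index 0.
; Alarm latches the Alarmed flag so the NPCAlarmed dispatch fires only once, passing along the instigator.
; Attack is a placeholder that only prints a debug string.
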(event `self.ReceiveAnyDamage`
  (params (Damage :type "Float (single-precision)") (DamageType :type "DamageType Object Reference") (InstigatedBy :type "Controller Object Reference") (DamageCauser :type "Actor Object Reference"))
  ;[1 1 1] Alarm by Damage
  (`parent.ReceiveAnyDamage` Damage DamageType InstigatedBy DamageCauser)
  (if (== InstigatedBy (`GameplayStatics.GetPlayerCharacter` 0))
    (`self.Alarm` (`GameplayStatics.GetPlayerCharacter` 0))))

(event `Attack`
  (params (Target :type "Actor Object Reference"))
  (`KismetSystemLibrary.PrintString` "Mob Actttack"))

(fn `Alarm`
  (params (Instigator :type "Pawn Object Reference"))
  (if (not (`self.Alarmed`))
    (set `self.Alarmed` true)
    (`self.NPCAlarmed` Instigator)))

(fn `UserConstructionScript`)