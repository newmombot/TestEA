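; AI controller for NPC characters that sets up follow behavior and listens for NPC events.
; On possess, it caches the pawn as an NPCCharacter, initializes NPCFollowComponent, and binds to the NPC's alarmed event and the component's destination-reached event.
; Reactions are placeholders: NPCAlarmed only prints a debug string, while FollowDestReached and NPCDead are empty.
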(event `self.OnPossess`
  (params (PossessedPawn :type "Pawn Object Reference"))
  (`self.Init`))

(fn `BindEvents`
  (add `/Game/Blueprints/NPC/NPCCharacter.NPCAlarmed` (`self.NPC`) (`|CreateDelegate` :!event `NPCAlarmed`))
  (add `/Game/Blueprints/NPC/Cmponents/NPC-FollowComponent.DestReached` (`self.NPC-FollowComponent`) (`|CreateDelegate` :!event `FollowDestReached`)))

(fn `FollowDestReached`)

(fn `Init`
  (bind _asnpccharacter (cast `/Game/Blueprints/NPC/NPCCharacter` (`self.K2_GetPawn`)))
  (set `self.NPC` _asnpccharacter)
  (`/Game/Blueprints/NPC/Cmponents/MainNPCContrlComponent.Init` (`self.NPC-FollowComponent`))
  (`self.BindEvents`))

(fn `NPCAlarmed`
  (params (Instigator :type "Pawn Object Reference"))
  (`KismetSystemLibrary.PrintString` "NPC Alarmed"))

(fn `NPCDead`)

(fn `UserConstructionScript`)